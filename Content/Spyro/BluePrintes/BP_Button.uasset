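; BP_Button is an interactive button that the Spyro player uses to open and close a referenced Door.
; Its Box overlap registers the button as the player's CurrentInteractiveObject and shows a text prompt, then clears both when the player leaves.
; The Interact event runs a FlipFlop that alternates between the Door's Open and Close.
; An author note plans to move the overlap and prompt logic into the parent, leaving only Interact here.
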(event `self.ReceiveBeginPlay`
  ;[1 1 1] Hacer que esto se haga en el padre y que solo sea la funcion de interact la que haga lo que tenga que hacer
  (`SceneComponent.SetVisibility` (`self.TextRender`) false false :!label _label))

(event `self.Box.OnComponentBeginOverlap`
  (params (OverlappedComponent :type "PrimitiveComponent Object Reference") (OtherActor :type "Actor Object Reference") (OtherComp :type "PrimitiveComponent Object Reference") (OtherBodyIndex :type Integer) (bFromSweep :type Boolean) (SweepResult :type "HitResult Structure (by ref)"))
  ;[1 1 1] Hacer que esto se haga en el padre y que solo sea la funcion de interact la que haga lo que tenga que hacer
  (bind _asbp_player_spyro (cast `/Game/Spyro/BluePrintes/BP_Player_Spyro` OtherActor))
  (set `/Game/Spyro/BluePrintes/BP_Player_Spyro.CurrentInteractiveObject` self _asbp_player_spyro)
  (`SceneComponent.SetVisibility` (`self.TextRender`) true false))

(event `self.Box.OnComponentEndOverlap`
  (params (OverlappedComponent :type "PrimitiveComponent Object Reference") (OtherActor :type "Actor Object Reference") (OtherComp :type "PrimitiveComponent Object Reference") (OtherBodyIndex :type Integer))
  ;[1 1 1] Hacer que esto se haga en el padre y que solo sea la funcion de interact la que haga lo que tenga que hacer
  (bind _asbp_player_spyro (cast `/Game/Spyro/BluePrintes/BP_Player_Spyro` OtherActor))
  (set `/Game/Spyro/BluePrintes/BP_Player_Spyro.CurrentInteractiveObject` null _asbp_player_spyro)
  (goto _label))

(event `self.Interact`
  (bind _door (`self.door`))
  (`/Engine/EditorBlueprintResources/StandardMacros.FlipFlop`
    (:`A`
      (`/Game/Spyro/BluePrintes/BP_Door.Open` _door))
    (:`B`
      (`/Game/Spyro/BluePrintes/BP_Door.Close` _door))))

(fn `UserConstructionScript`)