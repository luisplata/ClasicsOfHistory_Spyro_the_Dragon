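; Fire attack projectile for Spyro that flies along its local X axis at PowerVelocity and destroys itself after a five-second timer.
; Tick drives the movement, while hit and overlap events on Sphere1 share logic that scans the other actor's tags for "enemy".
; An enemy tag only prints a damage message, with no damage applied.
; Any tagged actor triggers self-destruction, while untagged actors do not.
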(event `self.ReceiveBeginPlay`
  (`KismetSystemLibrary.K2_SetTimerDelegate` (delegate `Destroy_Selft`) 5.0))

(event `Destroy_Selft`
  (`KismetSystemLibrary.PrintString` "Hello")
  (`self.K2_DestroyActor`))

(event `self.ReceiveTick`
  (params (DeltaSeconds :type "Float (single-precision)"))
  (`self.K2_AddActorLocalOffset` (`KismetMathLibrary.MakeVector` (* DeltaSeconds (`self.power_velocity`)))))

(event `self.Sphere1.OnComponentHit`
  (params (HitComponent :type "PrimitiveComponent Object Reference") (OtherActor :type "Actor Object Reference") (OtherComp :type "PrimitiveComponent Object Reference") (NormalImpulse :type "Vector Structure") (Hit :type "HitResult Structure (by ref)"))
  (for _array_element (`Actor.Tags` OtherActor)
    (if (== _array_element "enemy")
      (`KismetSystemLibrary.PrintString` "Hit one damage" :!label _label))
    (`self.Destroy_Selft` :!label _label_2)))

(event `self.Sphere1.OnComponentBeginOverlap`
  (params (OverlappedComponent :type "PrimitiveComponent Object Reference") (OtherActor :type "Actor Object Reference") (OtherComp :type "PrimitiveComponent Object Reference") (OtherBodyIndex :type Integer) (bFromSweep :type Boolean) (SweepResult :type "HitResult Structure (by ref)"))
  (for _array_element (`Actor.Tags` OtherActor)
    (if (== _array_element "enemy")
      (goto _label)
      (else
        (goto _label_2)))))

(fn `UserConstructionScript`)