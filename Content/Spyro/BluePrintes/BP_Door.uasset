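; BP_Door is a sliding door that other logic drives through its Open and Close events.
; A timeline plays or reverses, moving Cube1 along relative Y by the curve value times RotationValue, a translation despite the variable's name.
; A box trigger shows a text label while BP_Player_Spyro overlaps it and hides it on exit; the label starts hidden.
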(event `Open`
  (bind (_direction _curve) (`Timeline|Timeline` :!label _label)
    (:`Update`
      (`SceneComponent.K2_SetRelativeLocation` (`self.Cube1`) (`KismetMathLibrary.MakeVector` 0.0 (* _curve (`self.RotationValue`))) false false))))

(event `Close`
  (goto _label :!via `Reverse`))

(event `self.Box.OnComponentBeginOverlap`
  (params (OverlappedComponent :type "PrimitiveComponent Object Reference") (OtherActor :type "Actor Object Reference") (OtherComp :type "PrimitiveComponent Object Reference") (OtherBodyIndex :type Integer) (bFromSweep :type Boolean) (SweepResult :type "HitResult Structure (by ref)"))
  (cast `/Game/Spyro/BluePrintes/BP_Player_Spyro` OtherActor)
  (`SceneComponent.SetVisibility` (`self.TextRender`) true false))

(event `self.Box.OnComponentEndOverlap`
  (params (OverlappedComponent :type "PrimitiveComponent Object Reference") (OtherActor :type "Actor Object Reference") (OtherComp :type "PrimitiveComponent Object Reference") (OtherBodyIndex :type Integer))
  (cast `/Game/Spyro/BluePrintes/BP_Player_Spyro` OtherActor)
  (`SceneComponent.SetVisibility` (`self.TextRender`) false false))

(event `self.ReceiveBeginPlay`
  (`SceneComponent.SetVisibility` (`self.TextRender`) false false))

(fn `UserConstructionScript`)