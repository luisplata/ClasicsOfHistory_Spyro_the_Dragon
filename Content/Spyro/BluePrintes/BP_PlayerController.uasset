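; Player controller for the Spyro player character that routes the interact input to the object the character can currently use.
; It caches the possessed BP_Player_Spyro pawn on BeginPlay and re-fetches it on input if that reference is invalid.
; Pressing interact calls Interact on the pawn's CurrentInteractiveObject when one is valid.
; The pause input event is present but has no logic.
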(event `self.ReceiveBeginPlay`
  (bind _asbp_player_spyro (cast `/Game/Spyro/BluePrintes/BP_Player_Spyro` (`self.K2_GetPawn`)))
  (set `self.Player_Pawn` _asbp_player_spyro))

(event `EnhancedInput|/Game/Spyro/Input/IA_SPYRO_PAUSA`
  (params (ActionValue :type Boolean) (ElapsedSeconds :type "Float (double-precision)") (TriggeredSeconds :type "Float (double-precision)") (InputAction :type "InputAction Object Reference" :default "/Game/Spyro/Input/IA_SPYRO_PAUSA.IA_SPYRO_PAUSA")))

(event `EnhancedInput|/Game/Spyro/Input/IA_Pyro_Interact`
  (params (ActionValue :type Boolean) (ElapsedSeconds :type "Float (double-precision)") (TriggeredSeconds :type "Float (double-precision)") (InputAction :type "InputAction Object Reference" :default "/Game/Spyro/Input/IA_Pyro_Interact.IA_Pyro_Interact"))
  (bind _currentinteractiveobject (`/Game/Spyro/BluePrintes/BP_Player_Spyro.CurrentInteractiveObject` (`self.Player_Pawn`)))
  (:`Started`
    (`/Engine/EditorBlueprintResources/StandardMacros.IsValid` (`self.Player_Pawn`)
      (:`Is Valid`
        _)
      (:`Is Not Valid`
        (bind _asbp_player_spyro (cast `/Game/Spyro/BluePrintes/BP_Player_Spyro` (`self.K2_GetPawn`)))
        (set `self.Player_Pawn` _asbp_player_spyro)))
    (`/Engine/EditorBlueprintResources/StandardMacros.IsValid` _currentinteractiveobject
      (:`Is Valid`
        (`/Game/Spyro/BluePrintes/BP_Interactable.Interact` _currentinteractiveobject)))))

(fn `UserConstructionScript`)