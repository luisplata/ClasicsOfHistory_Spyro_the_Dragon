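; Game mode for the Spyro game that runs the intro and end cinematics.
; On BeginPlay it registers itself with GIBP_Sypro, plays Intro_02, waits its duration, then enables pausing and sets the player pawn's IsNotPaused flag.
; LoadEndCinematic clears both flags, plays Outro, then restores them after the same duration-based delay.
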(event `self.ReceiveBeginPlay`
  (bind _asgibp_sypro (cast `/Game/Spyro/BluePrintes/GIBP_Sypro` (`GameplayStatics.GetGameInstance`)))
  (set `/Game/Spyro/BluePrintes/GIBP_Sypro.GameMode` self _asgibp_sypro)
  (bind _asgibp_sypro_2 (cast `/Game/Spyro/BluePrintes/GIBP_Sypro` (`GameplayStatics.GetGameInstance`)))
  (set `/Game/Spyro/BluePrintes/GIBP_Sypro.GameMode` self _asgibp_sypro_2)
  (bind _outactor (`LevelSequencePlayer.CreateLevelSequencePlayer` "/Game/Spyro/Sequence/intro_02.intro_02"))
  (bind _sequenceplayer (`LevelSequenceActor.SequencePlayer` _outactor))
  (`MovieSceneSequencePlayer.Play` _sequenceplayer)
  (`KismetSystemLibrary.Delay` (`TimeManagementBlueprintLibrary.Conv_QualifiedFrameTimeToSeconds` (`MovieSceneSequencePlayer.GetDuration` _sequenceplayer)))
  (bind _asbp_player_controller (cast `/Game/Spyro/BluePrintes/BP_PlayerController` (`GameplayStatics.GetPlayerController` 0)))
  (set `/Game/Spyro/BluePrintes/BP_PlayerController.CanPause` true _asbp_player_controller)
  (bind _asbp_player_spyro (cast `/Game/Spyro/BluePrintes/BP_Player_Spyro` (`Controller.K2_GetPawn` _asbp_player_controller)))
  (set `/Game/Spyro/BluePrintes/BP_Player_Spyro.isNotPaused` true _asbp_player_spyro))

(event `LoadEndCinematic`
  (bind _asbp_player_controller (cast `/Game/Spyro/BluePrintes/BP_PlayerController` (`GameplayStatics.GetPlayerController` 0)))
  (set `/Game/Spyro/BluePrintes/BP_PlayerController.CanPause` false _asbp_player_controller)
  (bind _asbp_player_spyro (cast `/Game/Spyro/BluePrintes/BP_Player_Spyro` (`Controller.K2_GetPawn` _asbp_player_controller)))
  (set `/Game/Spyro/BluePrintes/BP_Player_Spyro.isNotPaused` false _asbp_player_spyro)
  (bind _outactor (`LevelSequencePlayer.CreateLevelSequencePlayer` "/Game/Spyro/Sequence/outro.outro"))
  (bind _sequenceplayer (`LevelSequenceActor.SequencePlayer` _outactor))
  (`MovieSceneSequencePlayer.Play` _sequenceplayer)
  (`KismetSystemLibrary.Delay` (`TimeManagementBlueprintLibrary.Conv_QualifiedFrameTimeToSeconds` (`MovieSceneSequencePlayer.GetDuration` _sequenceplayer)))
  (bind _asbp_player_controller_2 (cast `/Game/Spyro/BluePrintes/BP_PlayerController` (`GameplayStatics.GetPlayerController` 0)))
  (set `/Game/Spyro/BluePrintes/BP_PlayerController.CanPause` true _asbp_player_controller_2)
  (bind _asbp_player_spyro_2 (cast `/Game/Spyro/BluePrintes/BP_Player_Spyro` (`Controller.K2_GetPawn` _asbp_player_controller_2)))
  (set `/Game/Spyro/BluePrintes/BP_Player_Spyro.isNotPaused` true _asbp_player_spyro_2))

(fn `UserConstructionScript`)